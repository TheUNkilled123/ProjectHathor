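; Behavior tree decorator that checks whether a BP_EnemyBuff enemy is within its first attack range of its target.
; It passes when the distance from the controlled pawn to the blackboard Target actor is at most the enemy's AttackRange01.
; The pawn is cast to BP_EnemyBuff and cached in OwnerRef whenever that reference is invalid, then the check runs.
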(fn `PerformConditionCheckAI`
  (params (OwnerController :type "AIController Object Reference") (ControlledPawn :type "Pawn Object Reference"))
  (returns (ReturnValue :type Boolean))
  (if (`KismetSystemLibrary.IsValid` (`self.ownerRef`)) :!label _label
    (return (<= (`Actor.GetDistanceTo` ControlledPawn (`BTFunctionLibrary.GetBlackboardValueAsActor` (`self.Target`))) (`HathorAiCharacterBase.attackRange01` (`self.ownerRef`))))
    (else
      (bind _asbp_enemy_buff (cast `/Game/Blueprints/Characters/Enemies/BP_EnemyBuff` ControlledPawn))
      (set `self.ownerRef` _asbp_enemy_buff)
      (goto _label))))